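; Player pawn for a gold mining and refining game, routing J/K/L/R input by location while electricity is on.
; Cave logic is a timed random-key minigame whose points award gold with random traits.
; Fabric logic matches typed codes to alter those traits, and repeated failures switch location to no-electricity.
; Selling prices gold by traits and triggers the ending past a money target, with HUD widgets showing prompts, map and energy.
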(event Custom|RandomButtom
  ;[0.15 0.15 0.15 0.5] Event set timer
  (Variables|Buttons|SetrandomButton (Math|Random|RandomIntegerinRange 0 2))
  (CallFunction|-Points)
  (Default|SetRightClick (Variables|/Game/Project/Blueprints/UI/HUDMainLevel/BP_HUDMainLevel.BP_HUDMainLevel_C|GetWBP%20Cur%20Click (Variables|Links|GetAs%20BP%20HUDMain%20Level))))

(event Custom|Set%20timer%20by%20rundom%20buttom
  ;[0.15 0.15 0.15 0.5] Event set timer
  (bind _returnvalue (Utilities|Time|SetTimerbyEvent (delegate Custom|RandomButtom) 5.0 true))
  (Variables|Buttons|SettymerByRundomButton _returnvalue)
  (Default|SetRightClick (Variables|/Game/Project/Blueprints/UI/HUDMainLevel/BP_HUDMainLevel.BP_HUDMainLevel_C|GetWBP%20Cur%20Click (Variables|Links|GetAs%20BP%20HUDMain%20Level))))

(event Custom|MapUnConstrauct
  ;[0.15 0.15 0.15 0.5] Call events after mapping
  (if (Variables|Electricity(Genratorvar)|GetElectricity)
    (switch Utilities|FlowControl|Switch|SwitchonE_LocaitionInputMode (Variables|Default|GetLocaitionInput)
      (:NewEnumerator0
        (CallFunction|SetTimerbyRundomButtom)))))

(event Input|EnhancedActionEvents|EnhancedInputActionIA_ClickJ
  (params (ActionValue :type Boolean) (ElapsedSeconds :type Float%20%28double-precision%29) (TriggeredSeconds :type Float%20%28double-precision%29) (InputAction :type Input%20Action%20Object%20Reference :default "/Game/Project/Input/Actions/IA_ClickJ.IA_ClickJ"))
  ;[0.15 0.15 0.15 0.5] Main mehanic
  (if (Variables|Electricity(Genratorvar)|GetElectricity)
    (switch Utilities|FlowControl|Switch|SwitchonE_LocaitionInputMode (Variables|Default|GetLocaitionInput)
      (:NewEnumerator0
        (Utilities|CaveLogic))
      (:NewEnumerator1
        (Utilities|FabricLogic))
      (:NewEnumerator4
        (CallFunction|SetElctricity)))))

(event Input|EnhancedActionEvents|EnhancedInputActionIA_ClickK
  (params (ActionValue :type Boolean) (ElapsedSeconds :type Float%20%28double-precision%29) (TriggeredSeconds :type Float%20%28double-precision%29) (InputAction :type Input%20Action%20Object%20Reference :default "/Game/Project/Input/Actions/IA_ClickK.IA_ClickK"))
  ;[0.15 0.15 0.15 0.5] Main mehanic
  (if (Variables|Electricity(Genratorvar)|GetElectricity)
    (switch Utilities|FlowControl|Switch|SwitchonE_LocaitionInputMode (Variables|Default|GetLocaitionInput)
      (:NewEnumerator0
        (Utilities|CaveLogic) ; enters at K
      )
      (:NewEnumerator1
        (Utilities|FabricLogic) ; enters at K
      )
      (:NewEnumerator4
        (CallFunction|SetElctricity)))))

(event Input|EnhancedActionEvents|EnhancedInputActionIA_ClickL
  (params (ActionValue :type Boolean) (ElapsedSeconds :type Float%20%28double-precision%29) (TriggeredSeconds :type Float%20%28double-precision%29) (InputAction :type Input%20Action%20Object%20Reference :default "/Game/Project/Input/Actions/IA_ClickL.IA_ClickL"))
  ;[0.15 0.15 0.15 0.5] Main mehanic
  (if (Variables|Electricity(Genratorvar)|GetElectricity)
    (switch Utilities|FlowControl|Switch|SwitchonE_LocaitionInputMode (Variables|Default|GetLocaitionInput)
      (:NewEnumerator0
        (Utilities|CaveLogic) ; enters at L
      )
      (:NewEnumerator1
        (Utilities|FabricLogic) ; enters at L
      )
      (:NewEnumerator4
        (CallFunction|SetElctricity)))))

(event Input|EnhancedActionEvents|EnhancedInputActionIA_ClickR
  (params (ActionValue :type Boolean) (ElapsedSeconds :type Float%20%28double-precision%29) (TriggeredSeconds :type Float%20%28double-precision%29) (InputAction :type Input%20Action%20Object%20Reference :default "/Game/Project/Input/Actions/IA_ClickR.IA_ClickR"))
  ;[0.15 0.15 0.15 0.5] Main mehanic
  (if (Variables|Electricity(Genratorvar)|GetElectricity)
    (switch Utilities|FlowControl|Switch|SwitchonE_LocaitionInputMode (Variables|Default|GetLocaitionInput)
      (:NewEnumerator1
        (Utilities|FabricLogic) ; enters at Reset
      )
      (:NewEnumerator4
        (CallFunction|SetElctricity)))))

(event Input|EnhancedActionEvents|EnhancedInputActionIA_ToggleMap
  (params (ActionValue :type Boolean) (ElapsedSeconds :type Float%20%28double-precision%29) (TriggeredSeconds :type Float%20%28double-precision%29) (InputAction :type Input%20Action%20Object%20Reference :default "/Game/Project/Input/Actions/IA_ToggleMap.IA_ToggleMap"))
  (bind _as_bp_hudmain_level (Variables|Links|GetAs%20BP%20HUDMain%20Level))
  (bind _wbp_map (Variables|/Game/Project/Blueprints/UI/HUDMainLevel/BP_HUDMainLevel.BP_HUDMainLevel_C|GetWBP%20Map _as_bp_hudmain_level))
  ;[0.15 0.15 0.15 0.5] Add and remove Map
  (if (Variables|/Game/Project/Blueprints/UI/HUDMainLevel/Widgets/ForAll/WBP_Map.WBP_Map_C|GetMapIsOpen _wbp_map)
    (Default|CloseMap _wbp_map)
    (else
      (Default|AddMap _as_bp_hudmain_level))))

(event EventBeginPlay
  ;[0.15 0.15 0.15 0.5] Cast
  (bind _asbp_hudmain_level (Utilities|Casting|CastToBP_HUDMainLevel (HUD|GetHUD (Game|GetPlayerController 0))))
  (Variables|Links|SetAs%20BP%20HUDMain%20Level _asbp_hudmain_level)
  ;[0.15 0.15 0.15 0.5] Construct after map
  (CallFunction|MapUnConstrauct))

(fn ConstructionScript)

(fn -Points
  (Variables|Default|SetPoints (- (Variables|Default|GetPoints) 2))
  (if (< (Variables|Default|GetPoints) 0)
    (Variables|Default|SetPoints 0)))

(fn +Points
  (Variables|Default|SetPoints (+ (Variables|Default|GetPoints) 1)))

(fn +GeneratorEnergy
  (Default|+Energy (Variables|/Game/Project/Blueprints/UI/HUDMainLevel/BP_HUDMainLevel.BP_HUDMainLevel_C|GetWBP%20Generator%20Energy (Variables|Links|GetAs%20BP%20HUDMain%20Level))))

(fn AddRandomGold
  (bind _output_get (Variables|Golds(Cavevar)|SetGoldParam (Utilities|Struct|MakeS_Gold (Math|Random|RandomBool) (Math|Random|RandomBool) (Math|Random|RandomBool))))
  (Utilities|Array|Add (Variables|Golds(Cavevar)|GetArrayGolds) _output_get))

(fn SetCostGold
  (params (Gold :type S%20Gold%20Structure))
  (bind (_isnotpoluted _isshiny _isenriched) (Utilities|Struct|BreakS_Gold Gold))
  (bind _returnvalue (Math|Conversions|ToInteger(Boolean) _isenriched))
  (bind _returnvalue_2 (Math|Conversions|ToInteger(Boolean) _isnotpoluted))
  (bind _returnvalue_3 (Math|Conversions|ToInteger(Boolean) _isshiny))
  (bind _returnvalue_4 (+ _returnvalue_2 _returnvalue_3 _returnvalue))
  (bind _returnvalue_5 (* _returnvalue_4 100))
  (if (> _returnvalue_5 0)
    (return _returnvalue_5)
    (else
      (return 1))))

(fn SellGold
  (params (GoldsArray :type Array%20of%20S%20Gold%20Structures) (IndexGold :type Integer))
  (if (or (!= -1 IndexGold) (!= IndexGold 0))
    (bind _goldcost (CallFunction|SetCostGold (Utilities|Array|Get(acopy) GoldsArray IndexGold)))
    (Variables|Default|SetPlayersMoney (+ _goldcost (Variables|Default|GetPlayersMoney)))
    (Utilities|Array|RemoveIndex GoldsArray IndexGold)
    (if (> (Variables|Default|GetPlayersMoney) 5000)
      (Default|AddtheEnd (Variables|Links|GetAs%20BP%20HUDMain%20Level)))))

(fn SetElctricity
  (if (Variables|Electricity(Genratorvar)|GetElectricity)
    (Variables|Electricity(Genratorvar)|SetElectricity false)
    (else
      (Variables|Electricity(Genratorvar)|SetElectricity true))))